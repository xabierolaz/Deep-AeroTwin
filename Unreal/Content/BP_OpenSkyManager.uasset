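; BP_OpenSkyManager is a manager Blueprint that shows live telemetry from an HTTP endpoint as a single BP_AirplaneMarker.
; A looping timer sends a GET request through VaRest, with an in-flight flag preventing overlapping requests.
; On a successful response it spawns the marker if missing, blends the player's view to it, and updates its longitude, latitude, altitude and heading from the JSON.
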(event `self.ReceiveBeginPlay`
  (`KismetSystemLibrary.K2_SetTimerDelegate` (delegate `PolltELEMETRY`) (`self.PollInterval`) true))

(event `OnTelemetryResponse`
  (params (Request :type "VaRestRequestJSON Object Reference"))
  (bind _returnvalue (`VaRestRequestJSON.GetResponseObject` Request))
  (bind _droneactor (`self.DroneActor`))
  (bind _returnvalue_2 (`VaRestJsonObject.GetNumberField` _returnvalue "heading"))
  (bind _returnvalue_3 (`VaRestJsonObject.GetNumberField` _returnvalue "lon"))
  (bind _returnvalue_4 (`VaRestJsonObject.GetNumberField` _returnvalue "lat"))
  (bind _returnvalue_5 (`VaRestJsonObject.GetNumberField` _returnvalue "alt"))
  (if (== (`VaRestRequestJSON.GetResponseCode` Request) 200)
    (if (`KismetSystemLibrary.IsValid` (`self.DroneActor`))
      (`/Game/BP_AirplaneMarker.UpdateFromState` _droneactor _returnvalue_3 _returnvalue_4 _returnvalue_5 _returnvalue_2 "\"\"" "0" "\"\"")
      (set `self.RequestInFlight` false)
      (else
        (bind _returnvalue_6 (`|SpawnActorFromClass` "/Game/BP_AirplaneMarker.BP_AirplaneMarker_C" (`KismetMathLibrary.MakeTransform` (0.0 0.0 0.0)) "AlwaysSpawn" "MultiplyWithRoot" null null))
        (bind _output_get (set `self.DroneActor` _returnvalue_6))
        (`PlayerController.SetViewTargetWithBlend` (`GameplayStatics.GetPlayerController` 0) _output_get 0.2 "VTBlend_Linear" 0.0 false)
        (`KismetSystemLibrary.PrintString` "SPAWNED")
        (`/Game/BP_AirplaneMarker.UpdateFromState` _droneactor _returnvalue_3 _returnvalue_4 _returnvalue_5 _returnvalue_2 "\"\"" "0" "\"\"")
        (set `self.RequestInFlight` false)))
    (else
      (set `self.RequestInFlight` false))))

(event `PolltELEMETRY`
  (if (not (`self.RequestInFlight`))
    (set `self.RequestInFlight` true)
    (`VaRestSubsystem.CallURL` (subsystem `VaRestSubsystem`) (`self.EndpointURL`) "GET" "x_www_form_urlencoded_url" null (delegate `OnTelemetryResponse`))))

(fn `UserConstructionScript`)