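; BP_AirplaneMarker is an actor that represents an aircraft on a Cesium globe from reported state data.
; UpdateFromState moves its CesiumGlobeAnchor to the given longitude, latitude and altitude and applies heading as yaw, leaving callsign, last contact and ICAO unused.
; A TakeScreenshot event saves a high-resolution screenshot through a console command.
; The looping screenshot timer, DroneCapture scene capture and debug print are disconnected and never run.
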(event `self.ReceiveBeginPlay`)

(event `TakeScreenshot`
  (`KismetSystemLibrary.ExecuteConsoleCommand` "HighResShot 640x480 filename=raw_capture.png" null))

(fn `UpdateFromState`
  (params (lon :type "Float (double-precision)") (lat :type "Float (double-precision)") (alt :type "Float (double-precision)") (heading :type "Float (double-precision)") (callsign :type String) (lastContact :type String) (icao :type String))
  (`CesiumGlobeAnchorComponent.MoveToLongitudeLatitudeHeight` (`self.CesiumGlobeAnchor`) (`KismetMathLibrary.MakeVector` lon lat alt))
  (`self.K2_SetActorRotation` (`KismetMathLibrary.MakeRotator` 0.0 0.0 heading)))

(fn `UserConstructionScript`)